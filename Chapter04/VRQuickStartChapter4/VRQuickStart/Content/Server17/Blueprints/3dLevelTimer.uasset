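; A 3D level timer actor with a display widget that keeps turning to face the local player's camera.
; Each tick, UpdateRotation takes the look-at yaw from the first player camera to the DisplayWidget and flips it 180 degrees.
; Pitch and roll stay at zero, so the widget billboards only around the vertical axis.
; The graphs contain no timing logic, only this rotation.
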(event EventTick
  (params (DeltaSeconds :type Float%20%28single-precision%29))
  (CallFunction|UpdateRotation))

(fn ConstructionScript)

(fn UpdateRotation
  (bind _returnvalue (Game|GetPlayerCameraManager 0))
  (Utilities|IsValid _returnvalue
    (:Is%20Valid
      (Transformation|SetWorldRotation (Variables|Default|GetDisplayWidget) (Math|Rotator|MakeRotator 0.0 0.0 (+ (.yaw (Math|Rotator|FindLookatRotation (Camera|GetCameraLocation _returnvalue) (Transformation|GetWorldLocation (Variables|Default|GetDisplayWidget)))) 1.8e+02)) false false))))