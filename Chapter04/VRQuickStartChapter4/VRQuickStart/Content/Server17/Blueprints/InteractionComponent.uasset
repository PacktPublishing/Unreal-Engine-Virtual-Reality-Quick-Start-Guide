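; Interaction component that lets its owner focus, activate, hover, use, drag and pick up objects through interface messages.
; While enabled, each tick runs a gravity-curved, segmented line trace to track the focused actor and component, reporting enter, move and leave events.
; A sphere overlap picks the hover target for use, drag and pickup, with a second gate sending per-tick drag updates.
; Held objects attach to the component until dropped.
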(event Custom|Enable
  ;[1 1 1] Parabolic Line Tracing
  (Utilities|FlowControl|Gate false) ; enters at Open
)

(event Custom|Disable
  ;[1 1 1] Parabolic Line Tracing
  (Utilities|FlowControl|Gate false) ; enters at Close
)

(event Custom|ActivateUp
  (params (Instigator :type Pawn%20Object%20Reference))
  ;[1 1 1] Activation
  (Class|ObjectInteractionInterface|TraceActivateUp(Message) (Variables|Default|GetFocusObject) (Variables|Default|GetCurrentHit) Instigator))

(event Custom|ActivateDown
  (params (Instigator :type Pawn%20Object%20Reference))
  ;[1 1 1] Activation
  (Class|ObjectInteractionInterface|TraceActivateDown(Message) (Variables|Default|GetFocusObject) (Variables|Default|GetCurrentHit) Instigator))

(event Custom|StartDrag
  ;[1 1 1] Dragging
  (Variables|Default|SetDragging true)
  (Class|ButtonInteractionInterface|OnDragStart(Message) (Variables|Default|GetHoverObject) self)
  (Utilities|FlowControl|Gate true) ; enters at Open
)

(event Custom|EndDrag
  ;[1 1 1] Dragging
  (if (Variables|Default|GetDragging)
    (Variables|Default|SetDragging false)
    (Class|ButtonInteractionInterface|OnDragEnd(Message) (Variables|Default|GetHoverObject) self)
    (Utilities|FlowControl|Gate true) ; enters at Close
  ))

(event Custom|Pickup
  (bind _hoverobject (Variables|Default|GetHoverObject))
  ;[1 1 1] Pickup
  (Utilities|IsValid _hoverobject
    (:Is%20Valid
      (bind _pickup (Class|ButtonInteractionInterface|CanPickUp(Message) _hoverobject))
      (if _pickup
        (bind _output_get (Variables|Default|SetHeldObject (Variables|Default|GetHoverObject)))
        (Transformation|AttachComponentToComponent _output_get self "None" "KeepWorld" "KeepWorld" "KeepWorld" true)
        (Class|ButtonInteractionInterface|OnPickup(Message) (Variables|Default|GetHeldObject) self)))))

(event Custom|Drop
  ;[1 1 1] Dropping
  (Utilities|IsValid (Variables|Default|GetHeldObject)
    (:Is%20Valid
      (Transformation|DetachFromActor (Variables|Default|GetHeldObject) "KeepWorld" "KeepWorld" "KeepWorld")
      (Class|ButtonInteractionInterface|OnDrop(Message) (Variables|Default|GetHeldObject) self)
      (Variables|Default|SetHoverObject 0)
      (Variables|Default|SetHeldObject 0))))

(event Custom|UseHovered
  ;[1 1 1] Use Hovered
  (Class|ButtonInteractionInterface|OnUse(Message) (Variables|Default|GetHoverObject) self))

(event EventTick
  (params (DeltaSeconds :type Float%20%28single-precision%29))
  ;[1 1 1] Parabolic Line Tracing
  (Utilities|FlowControl|Gate false
    (:Exit
      (Utilities|FlowControl|Sequence
        (:then_0
          (bind _hit (CallFunction|ParabolicLineTrace 10 0.1 5e+02))
          (bind _output_get (Variables|Default|SetCurrentHit _hit))
          (CallFunction|InteractwithHit _output_get))
        (:then_1
          ;[1 1 1] Hovering
          (bind _outactors (Collision|SphereOverlapActors (Transformation|GetWorldLocation) (Variables|Default|GetInteractRadius) (Utilities|Array|MakeArray "ObjectTypeQuery2" "ObjectTypeQuery4") 0 (Utilities|Array|MakeArray (Components|GetOwner))))
          (if (!= (Utilities|Array|Get(acopy) _outactors) (Variables|Default|GetHoverObject))
            (Class|ButtonInteractionInterface|EndHover(Message) (Variables|Default|GetHoverObject) self)
            (CallFunction|EndDrag)
            (bind _output_get_2 (Variables|Default|SetHoverObject (Utilities|Array|Get(acopy) _outactors)))
            (Class|ButtonInteractionInterface|OnHover(Message) _output_get_2 self)))
        (:then_2
          ;[1 1 1] Dragging
          (Utilities|FlowControl|Gate true
            (:Exit
              (Class|ButtonInteractionInterface|OnDrag(Message) (Variables|Default|GetHoverObject) self))))))))

(fn InteractwithHit
  (params (Hit :type Hit%20Result%20Structure))
  ;[1 1 1] Initialize Variables
  (bind _output_get (LocalVariables|SetInHit Hit))
  (LocalVariables|SetInHitActor (.HitActor (Collision|BreakHitResult _output_get)))
  (LocalVariables|SetInHitComponent (.HitComponent (Collision|BreakHitResult _output_get)))
  ;[1 1 1] Are we looking at the same object?
  (if (== (Variables|Default|GetFocusObject) (LocalVariables|GetInHitActor))
    ;[1 1 1] Pass Component Information
    (Class|ObjectInteractionInterface|TraceMove(Message) (Variables|Default|GetFocusObject) (LocalVariables|GetInHit))
    (if (not (== (Variables|Default|GetFocusComponent) (LocalVariables|GetInHitComponent)))
      (Class|ObjectInteractionInterface|TraceLeaveComponent(Message) (Variables|Default|GetFocusObject) (LocalVariables|GetInHit) (Variables|Default|GetFocusComponent))
      (Class|ObjectInteractionInterface|TraceHitComponent(Message) (Variables|Default|GetFocusObject) (LocalVariables|GetInHit) (LocalVariables|GetInHitComponent))
      (Variables|Default|SetFocusComponent (LocalVariables|GetInHitComponent)))
    (else
      ;[1 1 1] Clear Variables
      (Class|ObjectInteractionInterface|TraceLeaveObject(Message) (Variables|Default|GetFocusObject) (LocalVariables|GetInHit))
      (Variables|Default|SetFocusObject 0)
      (Variables|Default|SetFocusComponent 0)
      (if (Utilities|DoesObjectImplementInterface (LocalVariables|GetInHitActor) "/Game/Server17/Blueprints/ObjectInteractionInterface.ObjectInteractionInterface_C")
        ;[1 1 1] Pass new Hit data
        (Class|ObjectInteractionInterface|TraceHitObject(Message) (LocalVariables|GetInHitActor) (LocalVariables|GetInHit))
        (Class|ObjectInteractionInterface|TraceHitComponent(Message) (LocalVariables|GetInHitActor) (LocalVariables|GetInHit) (LocalVariables|GetInHitComponent))
        (Variables|Default|SetFocusObject (LocalVariables|GetInHitActor))
        (Variables|Default|SetFocusComponent (LocalVariables|GetInHitComponent))))))

(fn ParabolicLineTrace
  (params (Steps :type Integer) (TimeStep :type Float%20%28single-precision%29) (Speed :type Float%20%28single-precision%29))
  ;[1 1 1] Initialize Variables
  (bind _output_get (LocalVariables|SetInitLoc (Transformation|GetWorldLocation)))
  (LocalVariables|SetPrevLoc _output_get)
  (LocalVariables|SetInSteps Steps)
  (LocalVariables|SetInTimeStep TimeStep)
  (LocalVariables|SetVelocity (* (Math|Vector|GetForwardVector) Speed))
  (bind _index (Utilities|FlowControl|ForLoopwithBreak 1 (LocalVariables|GetInSteps) :!label _label)
    (:LoopBody
      (bind (_outhit _returnvalue) (Collision|LineTraceByChannel (LocalVariables|GetPrevLoc) (+ (Math|Vector|MakeVector (* (.x (LocalVariables|GetVelocity)) (* _index (LocalVariables|GetInTimeStep))) (* (.y (LocalVariables|GetVelocity)) (* _index (LocalVariables|GetInTimeStep))) (- (* (.z (LocalVariables|GetVelocity)) (* _index (LocalVariables|GetInTimeStep))) (* (* _index (LocalVariables|GetInTimeStep)) (* _index (LocalVariables|GetInTimeStep)) 0.5 9.8e+02))) (LocalVariables|GetInitLoc)) "TraceTypeQuery1" false 0 "ForOneFrame"))
      (LocalVariables|SetPrevLoc (+ (Math|Vector|MakeVector (* (.x (LocalVariables|GetVelocity)) (* _index (LocalVariables|GetInTimeStep))) (* (.y (LocalVariables|GetVelocity)) (* _index (LocalVariables|GetInTimeStep))) (- (* (.z (LocalVariables|GetVelocity)) (* _index (LocalVariables|GetInTimeStep))) (* (* _index (LocalVariables|GetInTimeStep)) (* _index (LocalVariables|GetInTimeStep)) 0.5 9.8e+02))) (LocalVariables|GetInitLoc)))
      (LocalVariables|SetTempHit _outhit)
      (if _returnvalue
        (goto _label Break)))
    (:Completed
      (return (LocalVariables|GetTempHit)))))

(fn CanPickUp
  (return false))

(fn EndHover
  (params (Interactor :type Interaction%20Component%20Object%20Reference)))

(fn OnDrag
  (params (Interactor :type Interaction%20Component%20Object%20Reference))
  (return false))

(fn OnDragEnd
  (params (Interactor :type Interaction%20Component%20Object%20Reference))
  (return false))

(fn OnDragStart
  (params (Interactor :type Interaction%20Component%20Object%20Reference))
  (return false))

(fn OnDrop
  (params (Interactor :type Interaction%20Component%20Object%20Reference))
  (return false))

(fn OnHover
  (params (Interactor :type Interaction%20Component%20Object%20Reference)))

(fn OnPickup
  (params (Interactor :type Interaction%20Component%20Object%20Reference))
  (return false))

(fn OnUse
  (params (Interactor :type Interaction%20Component%20Object%20Reference))
  (return false))