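; Server17PlayerPawn is the VR player pawn, turning motion controller input into per-hand interactions with the world and widgets.
; Triggers drive each hand's InteractionComponent to activate, use hovered objects and drag, while also pressing its WidgetInteraction pointer as a left mouse click.
; Grips pick up and drop objects, and the left shoulder button toggles the tools menu.
; BeginPlay sets floor tracking origin; an Oculus-specific eye-level branch exists but never runs.
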(event EventBeginPlay
  ;[1 1 1] Set Tracking Origin based on player hardware
  (Class|HeadMountedDisplayFunctionLibrary|SetTrackingOrigin "Floor"))

(event Input|KeyboardEvents|MotionControllerLeftTrigger
  (params (Key :type Key%20Structure))
  (bind _self self)
  (bind _interactioncomponent_l (Variables|Default|GetInteractionComponent_L))
  (bind _interactioncomponent_l_2 (Variables|Default|GetInteractionComponent_L))
  (bind _widgetinteraction_l (Variables|Default|GetWidgetInteraction_L))
  ;[1 1 1] Activate Interaction Component
  (:Pressed
    (Default|ActivateDown _interactioncomponent_l_2 _self)
    ;[1 1 1] Hovering and Dragging
    (Default|UseHovered _interactioncomponent_l)
    (Default|StartDrag _interactioncomponent_l)
    ;[1 1 1] Widget Interaction
    (Class|WidgetInteractionComponent|PressPointerKey _widgetinteraction_l "LeftMouseButton"))
  (:Released
    (Default|ActivateUp _interactioncomponent_l_2 _self)
    (Default|EndDrag _interactioncomponent_l)
    (Class|WidgetInteractionComponent|ReleasePointerKey _widgetinteraction_l "LeftMouseButton")))

(event Input|KeyboardEvents|MotionControllerRightTrigger
  (params (Key :type Key%20Structure))
  (bind _self self)
  (bind _interactioncomponent_r (Variables|Default|GetInteractionComponent_R))
  (bind _interactioncomponent_r_2 (Variables|Default|GetInteractionComponent_R))
  (bind _widgetinteraction_r (Variables|Default|GetWidgetInteraction_R))
  ;[1 1 1] Activate Interaction Component
  (:Pressed
    (Default|ActivateDown _interactioncomponent_r_2 _self)
    ;[1 1 1] Hovering and Dragging
    (Default|UseHovered _interactioncomponent_r)
    (Default|StartDrag _interactioncomponent_r)
    ;[1 1 1] Widget Interaction
    (Class|WidgetInteractionComponent|PressPointerKey _widgetinteraction_r "LeftMouseButton"))
  (:Released
    (Default|ActivateUp _interactioncomponent_r_2 _self)
    (Default|EndDrag _interactioncomponent_r)
    (Class|WidgetInteractionComponent|ReleasePointerKey _widgetinteraction_r "LeftMouseButton")))

(event Input|KeyboardEvents|MotionControllerLeftGrip1
  (params (Key :type Key%20Structure))
  (bind _interactioncomponent_l (Variables|Default|GetInteractionComponent_L))
  ;[1 1 1] Grip Code
  (:Pressed
    (Default|Pickup _interactioncomponent_l))
  (:Released
    (Default|Drop _interactioncomponent_l)))

(event Input|KeyboardEvents|MotionControllerRightGrip1
  (params (Key :type Key%20Structure))
  (bind _interactioncomponent_r (Variables|Default|GetInteractionComponent_R))
  ;[1 1 1] Grip Code
  (:Pressed
    (Default|Pickup _interactioncomponent_r))
  (:Released
    (Default|Drop _interactioncomponent_r)))

(event Input|KeyboardEvents|MotionControllerLeftShoulder
  (params (Key :type Key%20Structure))
  ;[1 1 1] Toggle Tools Menu Visibility
  (:Pressed
    (Rendering|ToggleVisibility (Variables|Default|GetChildActor_ToolsWidget) false)))

(fn ConstructionScript)