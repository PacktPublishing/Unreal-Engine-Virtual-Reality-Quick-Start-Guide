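; StationButton is a pressable button actor that responds to trace-based interaction and shows its state by color.
; Trace callbacks tint the Cone's material Color parameter green on hover, red while pressed, and white when the trace leaves.
; Activate down sets the ButtonPressed flag, while release or leaving clears it.
; All trace handlers return false, and the component-level and move handlers do nothing else.
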(event EventBeginPlay)

(event Collision|EventActorBeginOverlap
  (params (OtherActor :type Actor%20Object%20Reference)))

(event EventTick
  (params (DeltaSeconds :type Float%20%28single-precision%29)))

(fn ConstructionScript)

(fn TraceActivateDown
  (params (Hit :type Hit%20Result%20Structure) (Instigator :type Pawn%20Object%20Reference))
  (Variables|Default|SetButtonPressed true)
  (Rendering|Material|SetVectorParameterValueonMaterials (Variables|Default|GetCone) "Color" "1.000000,0.000000,0.000000")
  (return false))

(fn TraceActivateUp
  (params (Hit :type Hit%20Result%20Structure) (Instigator :type Pawn%20Object%20Reference))
  (Rendering|Material|SetVectorParameterValueonMaterials (Variables|Default|GetCone) "Color" "0.000000,1.000000,0.000000")
  (Variables|Default|SetButtonPressed false)
  (return false))

(fn TraceHitComponent
  (params (Hit :type Hit%20Result%20Structure) (Component :type Primitive%20Component%20Object%20Reference))
  (return false))

(fn TraceHitObject
  (params (Hit :type Hit%20Result%20Structure))
  (Rendering|Material|SetVectorParameterValueonMaterials (Variables|Default|GetCone) "Color" "0.000000,1.000000, 0")
  (return false))

(fn TraceLeaveComponent
  (params (Hit :type Hit%20Result%20Structure) (Component :type Primitive%20Component%20Object%20Reference))
  (return false))

(fn TraceLeaveObject
  (params (Hit :type Hit%20Result%20Structure))
  (Rendering|Material|SetVectorParameterValueonMaterials (Variables|Default|GetCone) "Color" "1.000000,1.000000,1.000000")
  (Variables|Default|SetButtonPressed false)
  (return false))

(fn TraceMove
  (params (Hit :type Hit%20Result%20Structure%20%28by%20ref%29))
  (return false))