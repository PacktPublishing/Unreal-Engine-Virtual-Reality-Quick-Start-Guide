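; InteractButton is a physical push button that an overlapping component presses down, calling Pressed when fully depressed.
; The first component to overlap is tracked; its movement along the button root's local Z, clamped to a maximum, sets the button's depth.
; Without a tracked component, the button eases back to rest via VInterpTo.
; A DoOnce fires the press once, resetting only when PressAmount drops below the maximum.
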(event OnComponentBeginOverlap(Button)
  (params (OverlappedComponent :type Primitive%20Component%20Object%20Reference) (OtherActor :type Actor%20Object%20Reference) (OtherComp :type Primitive%20Component%20Object%20Reference) (OtherBodyIndex :type Integer) (bFromSweep :type Boolean) (SweepResult :type Hit%20Result%20Structure%20%28by%20ref%29))
  ;[1 1 1] Button Press Functionality
  (Utilities|IsValid (Variables|Default|GetOverlapComponent)
    (:Is%20Not%20Valid
      (bind _output_get (Variables|Default|SetOverlapComponent OtherComp))
      (Variables|Default|SetInitOverlapLoc (Transformation|GetWorldLocation _output_get)))))

(event OnComponentEndOverlap(Button)
  (params (OverlappedComponent :type Primitive%20Component%20Object%20Reference) (OtherActor :type Actor%20Object%20Reference) (OtherComp :type Primitive%20Component%20Object%20Reference) (OtherBodyIndex :type Integer))
  ;[1 1 1] Button Press Functionality
  (if (== OtherComp (Variables|Default|GetOverlapComponent))
    (Variables|Default|SetOverlapComponent 0)))

(event EventTick
  (params (DeltaSeconds :type Float%20%28single-precision%29))
  (bind _overlapcomponent (Variables|Default|GetOverlapComponent))
  (bind _buttonroot (Variables|Default|GetButtonRoot))
  ;[1 1 1] Button Animation
  (Utilities|FlowControl|Sequence
    (:then_0
      (Utilities|IsValid _overlapcomponent
        (:Is%20Valid
          (bind _output_get (Variables|Default|SetPressAmount (Math|Float|Clamp(Float) (.z (- (Math|Transform|InverseTransformLocation (Transformation|GetWorldTransform _buttonroot) (Variables|Default|GetInitOverlapLoc)) (Math|Transform|InverseTransformLocation (Transformation|GetWorldTransform _buttonroot) (Transformation|GetWorldLocation _overlapcomponent)))) 0.0 (Variables|Default|GetMaxPressAmount))))
          (Transformation|SetRelativeLocation (Variables|Default|GetButton) (Math|Vector|MakeVector 0.0 0.0 (* _output_get -1.0)) false false))
        (:Is%20Not%20Valid
          (Transformation|SetRelativeLocation (Variables|Default|GetButton) (Math|Interpolation|VInterpTo (Variables|/Script/Engine.SceneComponent|GetRelativeLocation (Variables|Default|GetButton)) "0, 0,5.000000" DeltaSeconds 1e+01) false false))))
    (:then_1
      ;[1 1 1] What happens when the button is pressed?
      (if (>= (Variables|Default|GetPressAmount) (Variables|Default|GetMaxPressAmount))
        (Utilities|FlowControl|DoOnce false :!label _label
          (:Completed
            (Default|CallPressed)))
        (else
          (goto _label Reset))))))

(fn ConstructionScript)