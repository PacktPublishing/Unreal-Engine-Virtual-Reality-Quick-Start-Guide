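; InteractCube is an interactable physics cube that can be picked up and gives color feedback to traces.
; Pickup is gated by PickUpActive, with physics simulation switched off on pickup and back on when dropped.
; Trace callbacks set the material Color parameter to red on hit, green on press, red on release and white on leave.
; Hover, drag, use and remaining trace handlers are stubs, and an upward impulse is left unconnected.
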(event EventBeginPlay)

(event Collision|EventActorBeginOverlap
  (params (OtherActor :type Actor%20Object%20Reference)))

(event EventTick
  (params (DeltaSeconds :type Float%20%28single-precision%29)))

(fn ConstructionScript)

(fn CanPickUp
  (return (Variables|Default|GetPickUpActive)))

(fn EndHover
  (params (Interactor :type Interaction%20Component%20Object%20Reference))
  (return false))

(fn OnDrag
  (params (Interactor :type Interaction%20Component%20Object%20Reference))
  (return false))

(fn OnDragEnd
  (params (Interactor :type Interaction%20Component%20Object%20Reference))
  (return false))

(fn OnDragStart
  (params (Interactor :type Interaction%20Component%20Object%20Reference))
  (return false))

(fn OnDrop
  (params (Interactor :type Interaction%20Component%20Object%20Reference))
  (Physics|SetSimulatePhysics (Variables|Default|GetCube) true)
  (return false))

(fn OnHover
  (params (Interactor :type Interaction%20Component%20Object%20Reference))
  (return false))

(fn OnPickup
  (params (Interactor :type Interaction%20Component%20Object%20Reference))
  (Physics|SetSimulatePhysics (Variables|Default|GetCube) false)
  (return false))

(fn OnUse
  (params (Interactor :type Interaction%20Component%20Object%20Reference))
  (return false))

(fn TraceActivateDown
  (params (Hit :type Hit%20Result%20Structure) (Instigator :type Pawn%20Object%20Reference))
  (Rendering|Material|SetVectorParameterValueonMaterials (Variables|Default|GetCube) "Color" "0.000000,1.000000, 0")
  (return false))

(fn TraceActivateUp
  (params (Hit :type Hit%20Result%20Structure) (Instigator :type Pawn%20Object%20Reference))
  (Rendering|Material|SetVectorParameterValueonMaterials (Variables|Default|GetCube) "Color" "1.000000, 0, 0")
  (return false))

(fn TraceHitComponent
  (params (Hit :type Hit%20Result%20Structure) (Component :type Primitive%20Component%20Object%20Reference))
  (return false))

(fn TraceHitObject
  (params (Hit :type Hit%20Result%20Structure))
  (Rendering|Material|SetVectorParameterValueonMaterials (Variables|Default|GetCube) "Color" "1.000000, 0, 0")
  (return false))

(fn TraceLeaveComponent
  (params (Hit :type Hit%20Result%20Structure) (Component :type Primitive%20Component%20Object%20Reference))
  (return false))

(fn TraceLeaveObject
  (params (Hit :type Hit%20Result%20Structure))
  (Rendering|Material|SetVectorParameterValueonMaterials (Variables|Default|GetCube) "Color" "1.000000,1.000000,1.000000")
  (return false))

(fn TraceMove
  (params (Hit :type Hit%20Result%20Structure%20%28by%20ref%29))
  (return false))