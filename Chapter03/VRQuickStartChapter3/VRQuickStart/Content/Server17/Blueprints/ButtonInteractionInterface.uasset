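; ButtonInteractionInterface declares the calls an interactor can make on an interactable object, by its name a button.
; It covers hover start and end, pickup and drop, drag start, update and end, and use, each receiving the Interactor.
; A separate CanPickUp query takes no Interactor.
; Every function has a return value and only a stub body returning false, so behavior is left to implementers.
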(fn OnHover
  (params (Interactor :type Interaction%20Component%20Object%20Reference))
  (return false))

(fn EndHover
  (params (Interactor :type Interaction%20Component%20Object%20Reference))
  (return false))

(fn OnPickup
  (params (Interactor :type Interaction%20Component%20Object%20Reference))
  (return false))

(fn OnDrop
  (params (Interactor :type Interaction%20Component%20Object%20Reference))
  (return false))

(fn OnDrag
  (params (Interactor :type Interaction%20Component%20Object%20Reference))
  (return false))

(fn OnDragStart
  (params (Interactor :type Interaction%20Component%20Object%20Reference))
  (return false))

(fn OnDragEnd
  (params (Interactor :type Interaction%20Component%20Object%20Reference))
  (return false))

(fn CanPickUp
  (return false))

(fn OnUse
  (params (Interactor :type Interaction%20Component%20Object%20Reference))
  (return false))