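; Test puzzle actor that chains button presses to unlock pickup on drawer cubes, built from child InteractCube and InteractButton actors.
; On BeginPlay it casts each child actor, disables pickup on the step 2 and step 3 drawer cubes, and binds both buttons' Pressed events.
; The step 1 button re-enables the step 2 cube, and the step 2 button the step 3 cube.
; The StolenData cube is tinted green through a material parameter.
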(event Custom|UnlockStep2
  (Variables|/Game/Server17/Blueprints/InteractCube.InteractCube_C|SetPickUpActive (stale EventBeginPlay _asinteract_cube) true))

(event Custom|UnlockStep3
  (Variables|/Game/Server17/Blueprints/InteractCube.InteractCube_C|SetPickUpActive (stale EventBeginPlay _asinteract_cube_2) true))

(event EventBeginPlay
  (Utilities|FlowControl|Sequence
    (:then_0
      (bind _asinteract_cube (Utilities|Casting|CastToInteractCube (Variables|/Script/Engine.ChildActorComponent|GetChildActor (Variables|Default|GetFrontDrawerTest_Step2))))
      (Variables|/Game/Server17/Blueprints/InteractCube.InteractCube_C|SetPickUpActive _asinteract_cube false))
    (:then_1
      (bind _asinteract_cube_2 (Utilities|Casting|CastToInteractCube (Variables|/Script/Engine.ChildActorComponent|GetChildActor (Variables|Default|GetDrawerTest_Step3))))
      (Variables|/Game/Server17/Blueprints/InteractCube.InteractCube_C|SetPickUpActive _asinteract_cube_2 false))
    (:then_2
      (bind _asinteract_button (Utilities|Casting|CastToInteractButton (Variables|/Script/Engine.ChildActorComponent|GetChildActor (Variables|Default|GetButton_Step1))))
      (EventDispatchers|BindEventtoPressed _asinteract_button (delegate Custom|UnlockStep2)))
    (:then_3
      (bind _asinteract_button_2 (Utilities|Casting|CastToInteractButton (Variables|/Script/Engine.ChildActorComponent|GetChildActor (Variables|Default|GetButtonStep2))))
      (EventDispatchers|BindEventtoPressed _asinteract_button_2 (delegate Custom|UnlockStep3)))
    (:then_4
      (bind _asinteract_cube_3 (Utilities|Casting|CastToInteractCube (Variables|/Script/Engine.ChildActorComponent|GetChildActor (Variables|Default|GetStolenData))))
      (Rendering|Material|SetVectorParameterValueonMaterials (Variables|/Game/Server17/Blueprints/InteractCube.InteractCube_C|GetCube _asinteract_cube_3) "Color" "0,1.000000, 0"))))

(fn ConstructionScript)