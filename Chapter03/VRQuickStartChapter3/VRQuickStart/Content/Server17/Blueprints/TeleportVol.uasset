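; TeleportVol is a teleport volume that moves a player to a point picked by a trace, apparently for VR-style locomotion.
; Trace callbacks show the TeleportViz marker on hit, move it with the hit location and hide it on leave.
; Releasing activation teleports the instigator to the hit XY at the volume's Z.
; Teleport adds the pawn-to-camera horizontal offset, so the camera, not the pawn origin, lands over the target.
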(event EventBeginPlay)

(event Collision|EventActorBeginOverlap
  (params (OtherActor :type Actor%20Object%20Reference)))

(event EventTick
  (params (DeltaSeconds :type Float%20%28single-precision%29)))

(fn ConstructionScript)

(fn Teleport
  (params (Player :type Pawn%20Object%20Reference) (Loc :type Vector))
  (bind _asplayer_controller (Utilities|Casting|CastToPlayerController (Pawn|GetController Player)))
  (Transformation|SetActorLocation Player (+ (Math|Vector|MakeVector (.x (- (Transformation|GetActorLocation Player) (Camera|GetCameraLocation (Variables|/Script/Engine.PlayerController|GetPlayerCameraManager _asplayer_controller)))) (.y (- (Transformation|GetActorLocation Player) (Camera|GetCameraLocation (Variables|/Script/Engine.PlayerController|GetPlayerCameraManager _asplayer_controller)))) 0.0) Loc) false false))

(fn TraceActivateDown
  (params (Hit :type Hit%20Result%20Structure) (Instigator :type Pawn%20Object%20Reference))
  (return false))

(fn TraceActivateUp
  (params (Hit :type Hit%20Result%20Structure) (Instigator :type Pawn%20Object%20Reference))
  (bind _location (Collision|BreakHitResult Hit))
  (CallFunction|Teleport Instigator (Math|Vector|MakeVector (.x _location) (.y _location) (.z (Transformation|GetActorLocation))))
  (return false))

(fn TraceHitComponent
  (params (Hit :type Hit%20Result%20Structure) (Component :type Primitive%20Component%20Object%20Reference))
  (return false))

(fn TraceHitObject
  (params (Hit :type Hit%20Result%20Structure))
  (Rendering|SetVisibility (Variables|Default|GetTeleportViz) true true)
  (return false))

(fn TraceLeaveComponent
  (params (Hit :type Hit%20Result%20Structure) (Component :type Primitive%20Component%20Object%20Reference))
  (return false))

(fn TraceLeaveObject
  (params (Hit :type Hit%20Result%20Structure))
  (Rendering|SetVisibility (Variables|Default|GetTeleportViz) false true)
  (return false))

(fn TraceMove
  (params (Hit :type Hit%20Result%20Structure%20%28by%20ref%29))
  (Transformation|SetWorldLocation (Variables|Default|GetTeleportViz) (.Location (Collision|BreakHitResult Hit)) false false)
  (return false))